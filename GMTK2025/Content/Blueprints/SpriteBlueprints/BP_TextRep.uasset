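; BP_TextRep is a sprite Blueprint that represents a directional command and moves the player in that direction.
; Its OnComponentContinueOverlapping event prints the object name, then switches on Action to call the matching Up, Down, Right or Left move on PlayerRef.
; The sprite's begin-overlap event is empty, and a cast to BP_LoopBoxRep leading into the same logic is left disconnected.
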(event OnComponentBeginOverlap(PaperSprite)
  (params (OverlappedComponent :type Primitive%20Component%20Object%20Reference) (OtherActor :type Actor%20Object%20Reference) (OtherComp :type Primitive%20Component%20Object%20Reference) (OtherBodyIndex :type Integer) (bFromSweep :type Boolean) (SweepResult :type Hit%20Result%20Structure%20%28by%20ref%29)))

(event Custom|OnComponentContinueOverlapping
  (bind _playerref (Variables|Default|GetPlayerRef))
  (Development|PrintString (Utilities|GetObjectName self))
  (switch Utilities|FlowControl|Switch|SwitchonEAction (Variables|Default|GetAction)
    (:NewEnumerator0
      (Default|ActionMoveUp _playerref))
    (:NewEnumerator1
      (Default|ActionMoveDown _playerref))
    (:NewEnumerator2
      (Default|ActionMoveRight (Variables|Default|GetPlayerRef)))
    (:NewEnumerator3
      (Default|ActionMoveLeft _playerref))))

(event EventBeginPlay)

(event Collision|EventActorBeginOverlap
  (params (OtherActor :type Actor%20Object%20Reference)))

(event EventTick
  (params (DeltaSeconds :type Float%20%28single-precision%29)))

(fn ConstructionScript)